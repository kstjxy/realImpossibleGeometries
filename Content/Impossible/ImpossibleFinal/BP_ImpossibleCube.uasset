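; BP_ImpossibleCube is an impossible cube actor built from twelve pieces grouped into Back, Mid and Front sections.
; Init, run from both the construction script and BeginPlay, adds the pieces to their section arrays.
; It then sets custom depth stencil value 1 on the Front and Back pieces, leaving the Mid pieces untouched.
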(event EventBeginPlay
  (CallFunction|Init))

(event Collision|EventActorBeginOverlap
  (params (OtherActor :type Actor%20Object%20Reference)))

(event EventTick
  (params (DeltaSeconds :type Float%20%28single-precision%29)))

(fn ConstructionScript
  (CallFunction|Init))

(fn Init
  (bind _back (Variables|Default|GetBack))
  (bind _mid (Variables|Default|GetMid))
  (bind _front (Variables|Default|GetFront))
  ;[1 1 1] Organize all elements of the cube into different sections for convenience
  (Utilities|Array|Add _back (Variables|Default|GetBack1))
  (Utilities|Array|Add _back (Variables|Default|GetBack2))
  (Utilities|Array|Add _back (Variables|Default|GetBack3))
  (Utilities|Array|Add _mid (Variables|Default|GetMid1))
  (Utilities|Array|Add _mid (Variables|Default|GetMid2))
  (Utilities|Array|Add _mid (Variables|Default|GetMid3))
  (Utilities|Array|Add _mid (Variables|Default|GetMid4))
  (Utilities|Array|Add _mid (Variables|Default|GetMid5))
  (Utilities|Array|Add _mid (Variables|Default|GetMid6))
  (Utilities|Array|Add _front (Variables|Default|GetFront1))
  (Utilities|Array|Add _front (Variables|Default|GetFront2))
  (Utilities|Array|Add _front (Variables|Default|GetFront3))
  (for _array_element (Variables|Default|GetFront)
    (Rendering|SetCustomDepthStencilValue _array_element 1))
  (for _array_element_2 (Variables|Default|GetBack)
    (Rendering|SetCustomDepthStencilValue _array_element_2 1)))