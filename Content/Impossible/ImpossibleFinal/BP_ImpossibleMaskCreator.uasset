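; BP_ImpossibleMaskCreator sets up scene-capture masks for the impossible cubes in the level.
; On BeginPlay it gathers every BP_ImpossibleCube and fills two capture show-only lists from their column components.
; The back capture renders Back and Mid columns, with Mid occluding the ends, while the front capture renders only Front columns.
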(event EventBeginPlay
  (CallFunction|Init))

(event Collision|EventActorBeginOverlap
  (params (OtherActor :type Actor%20Object%20Reference)))

(event EventTick
  (params (DeltaSeconds :type Float%20%28single-precision%29)))

(fn ConstructionScript)

(fn Init
  (bind _back_capture (Variables|Default|GetBack%20Capture))
  (bind _outactors (Actor|GetAllActorsOfClass "/Game/Impossible/ImpossibleFinal/BP_ImpossibleCube.BP_ImpossibleCube_C"))
  (bind _output_get (Variables|Default|SetImpossibleCubes _outactors))
  (for _array_element _output_get ; For each cube in the level
    (for _array_element_2 (Variables|/Game/Impossible/ImpossibleFinal/BP_ImpossibleCube.BP_ImpossibleCube_C|GetBack _array_element)
      (Rendering|SceneCapture|ShowOnlyComponent _back_capture _array_element_2) ; Show only back columns in back capture mask
    )
    (for _array_element_3 (Variables|/Game/Impossible/ImpossibleFinal/BP_ImpossibleCube.BP_ImpossibleCube_C|GetMid _array_element)
      (Rendering|SceneCapture|ShowOnlyComponent _back_capture _array_element_3) ; Show mid columns in back capture to occlude ends
    )
    (for _array_element_4 (Variables|/Game/Impossible/ImpossibleFinal/BP_ImpossibleCube.BP_ImpossibleCube_C|GetFront _array_element)
      (Rendering|SceneCapture|ShowOnlyComponent (Variables|Default|GetFront%20Capture) _array_element_4) ; Show front columns in front capture mask
    )))