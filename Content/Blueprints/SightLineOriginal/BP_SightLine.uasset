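; Sight-line visibility actor that follows the first actor of ClassToFollow and maps what is visible around it.
; Each tick it fires a 360-degree fan of Visibility traces, ignoring that class, and stretches one VisSlice mesh instance per ray to the hit distance.
; An orthographic scene capture sits just below the slices, sized to CheckRange.
; MPC_SightLine receives the actor location, mask height and texture scale for materials.
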(event Custom|SightTrace
  (bind _returnvalue (Transformation|GetActorLocation))
  (bind _tracecount (Variables|Default|GetTraceCount))
  (for _index (range 0 (- _tracecount 1))
    (bind _output_get (Variables|Default|SetCurrentTraceStep _index))
    (bind (_outhit _returnvalue_2) (Collision|LineTraceByChannel _returnvalue (+ _returnvalue (* (Math|Vector|RotateVector (Transformation|GetActorForwardVector) (Math|Rotator|MakeRotator 0.0 0.0 (* (Math|Conversions|ToFloat(Integer) _output_get) (/ 3.6e+02 (Math|Conversions|ToFloat(Integer) _tracecount))))) (Variables|Default|GetCheckRange))) "TraceTypeQuery1" false (Variables|Default|GetActorsToIgnore) "None" true "(R=0.000000,G=1.000000,B=0.000000,A=1.000000)" "(R=1.000000,G=0.000000,B=0.000000,A=1.000000)" 0.1))
    (Components|InstancedStaticMesh|UpdateInstanceTransform (Variables|Default|GetVisSlice) (Variables|Default|GetCurrentTraceStep) (Math|Transform|MakeTransform (Math|Vector|SelectVector (Math|Vector|MakeVector 0.0 0.0 (Variables|Default|GetVisSliceHeightOffset)) "0, 0, 0" (Variables|Default|GetOffsetByHeight)) (Math|Rotator|FindLookatRotation (.TraceStart (Collision|BreakHitResult _outhit)) (.TraceEnd (Collision|BreakHitResult _outhit))) (Math|Vector|MakeVector (* (Math|Vector|VectorLength (- (Math|Vector|SelectVector (.Location (Collision|BreakHitResult _outhit)) (.TraceEnd (Collision|BreakHitResult _outhit)) _returnvalue_2) (.TraceStart (Collision|BreakHitResult _outhit)))) (Variables|Default|GetTraceHitOffset)) (* (* (Math|Vector|VectorLength (- (Math|Vector|SelectVector (.Location (Collision|BreakHitResult _outhit)) (.TraceEnd (Collision|BreakHitResult _outhit)) _returnvalue_2) (.TraceStart (Collision|BreakHitResult _outhit)))) (Variables|Default|GetTraceHitOffset)) (/ 3.6e+02 (Math|Conversions|ToFloat(Integer) (Variables|Default|GetTraceCount)))) (* (Math|Vector|VectorLength (- (Math|Vector|SelectVector (.Location (Collision|BreakHitResult _outhit)) (.TraceEnd (Collision|BreakHitResult _outhit)) _returnvalue_2) (.TraceStart (Collision|BreakHitResult _outhit)))) (Variables|Default|GetTraceHitOffset)))) false true true)))

(event Custom|InitializeVisSlice
  (bind _scenecapturecomponent2d (Variables|Default|GetSceneCaptureComponent2D))
  (Components|InstancedStaticMesh|ClearInstances (Variables|Default|GetVisSlice))
  (for _index (range 0 (- (Variables|Default|GetTraceCount) 1))
    (Components|InstancedStaticMesh|AddInstance (Variables|Default|GetVisSlice) (Math|Transform|MakeTransform "0, 0, 0")))
  (CallFunction|SightTrace)
  (Variables|/Script/Engine.SceneCaptureComponent2D|SetOrthoWidth _scenecapturecomponent2d (Variables|Default|GetCheckRange))
  (Transformation|SetRelativeTransform _scenecapturecomponent2d (Math|Transform|MakeTransform (Math|Vector|MakeVector 0.0 0.0 (- (Variables|Default|GetVisSliceHeightOffset) 1.0)) "90.000000, 0, 0" "1,-1.000000,-1.000000") false false)
  (Rendering|Material|SetScalarParameterValue "/Game/Blueprints/SightLineOriginal/MPC_SightLine.MPC_SightLine" "SightLineMaskHeight" (+ (.z (Transformation|GetActorLocation)) (Variables|Default|GetVisSliceHeightOffset) -5e+02) :!class /Script/Engine.KismetMaterialLibrary)
  (Rendering|Material|SetScalarParameterValue "/Game/Blueprints/SightLineOriginal/MPC_SightLine.MPC_SightLine" "SightLineTexScale" (Variables|Default|GetCheckRange) :!class /Script/Engine.KismetMaterialLibrary)
  (Rendering|Material|SetVectorParameterValue "/Game/Blueprints/SightLineOriginal/MPC_SightLine.MPC_SightLine" "SightLineActorLocation" (Math|Conversions|ToLinearColor(Vector) (Transformation|GetActorLocation)) :!class /Script/Engine.KismetMaterialLibrary))

(event EventBeginPlay
  (CallFunction|InitializeVisSlice)
  (bind _outactors (Actor|GetAllActorsOfClass (Variables|Default|GetClassToFollow)))
  (Variables|Default|SetActorsToIgnore _outactors)
  (Variables|Default|SetActorToFollow (Utilities|Array|Get(acopy) _outactors)))

(event Collision|EventActorBeginOverlap
  (params (OtherActor :type Actor%20Object%20Reference)))

(event EventTick
  (params (DeltaSeconds :type Float%20%28single-precision%29))
  (bind _actortofollow (Variables|Default|GetActorToFollow))
  (Utilities|IsValid _actortofollow
    (:Is%20Valid
      (Transformation|SetActorLocation (Transformation|GetActorLocation _actortofollow) false false)
      (CallFunction|SightTrace)
      (Rendering|Material|SetVectorParameterValue "/Game/Blueprints/SightLineOriginal/MPC_SightLine.MPC_SightLine" "SightLineActorLocation" (Math|Conversions|ToLinearColor(Vector) (Transformation|GetActorLocation)) :!class /Script/Engine.KismetMaterialLibrary))))

(fn ConstructionScript
  (CallFunction|InitializeVisSlice))